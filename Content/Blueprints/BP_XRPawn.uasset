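; VR player pawn with navmesh-validated arc teleport, snap turning, input-driven hand poses and interaction with InteractiveActors.
; A right-hand line trace sets the hovered object, which can be held, rotated or destroyed, and shows its data in WBP_UI.
; The scale-animated widget lists spawnable classes and takes thumbstick and click input as simulated key presses through WidgetInteraction.
; Niagara point arrays draw the pointer and teleport traces.
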(event EventBeginPlay
  (bind _returnvalue (Game|GetPlayerController 0))
  (bind _returnvalue_2 (PlayerController|LocalPlayerSubsystems|GetEnhancedInputLocalPlayerSubsystem _returnvalue))
  (if (Class|HeadMountedDisplayFunctionLibrary|IsHeadMountedDisplayEnabled)
    (Class|HeadMountedDisplayFunctionLibrary|SetTrackingOrigin "LocalFloor")
    (Development|ExecuteConsoleCommand "xr.SecondaryScreenPercentage.HMDRenderTarget 100" 0)
    (Input|AddMappingContext _returnvalue_2 "/Game/Input/IMC_Default.IMC_Default" 0 "(bIgnoreAllPressedKeysUntilRelease=True,bForceImmediately=False,bNotifyUserSettings=False)")
    (Input|AddMappingContext _returnvalue_2 "/Game/Input/IMC_Hands.IMC_Hands" 0 "(bIgnoreAllPressedKeysUntilRelease=True,bForceImmediately=False,bNotifyUserSettings=False)")
    (Class|XRLoadingScreenFunctionLibrary|HideLoadingScreen)
    (Variables|Default|SetWidgetObject (.AsWBP%20UI (Utilities|Casting|CastToWBP_UI (UserInterface|GetUserWidgetObject (Variables|Default|GetWidget)))))
    (CallFunction|AddSpawnableObjectstoUI)
    (EventDispatchers|AssignOnObjectSpawnRequested (Variables|Default|GetWidgetObject) (EventDispatchers|CreateEvent :!event SpawnSelectedObject))
    (EventDispatchers|AssignOnObjectDestroyRequested (Variables|Default|GetWidgetObject) (EventDispatchers|CreateEvent :!event DestroyAvailableObject))
    (EventDispatchers|AssignOnFocusResetRequested (Variables|Default|GetWidgetObject) (EventDispatchers|CreateEvent :!event ResetWidgetFocus))
    (Components|Timeline|SetNewTime (Variables|Default|GetWidgetScaleTimeline) 0.0)))

(event Input|EnhancedActionEvents|EnhancedInputActionIA_ShowUI
  (params (ActionValue :type Boolean) (ElapsedSeconds :type Float%20%28double-precision%29) (TriggeredSeconds :type Float%20%28double-precision%29) (InputAction :type Input%20Action%20Object%20Reference :default "/Game/Input/IA_ShowUI.IA_ShowUI"))
  (:Started
    (Utilities|FlowControl|Sequence
      (:then_0
        (Utilities|FlowControl|DoOnce false
          (:Completed
            (CallFunction|ResetWidgetFocus))))
      (:then_1
        (bind _newscale (Timeline|WidgetScaleTimeline Play)
          (:Update
            (Transformation|SetWorldScale3D (Variables|Default|GetWidget) (Math|Conversions|ToVector(Float) _newscale)))))))
  (:Completed
    (Timeline|WidgetScaleTimeline Reverse)))

(event Input|EnhancedActionEvents|EnhancedInputActionIA_NavigateUI
  (params (ActionValue :type Vector%202D%20Structure) (ElapsedSeconds :type Float%20%28double-precision%29) (TriggeredSeconds :type Float%20%28double-precision%29) (InputAction :type Input%20Action%20Object%20Reference :default "/Game/Input/IA_NavigateUI.IA_NavigateUI"))
  (:Started
    (Class|WidgetInteractionComponent|PressandReleaseKey (Variables|Default|GetWidgetInteraction) (CallFunction|ThumbstickValuetoKeyboardKey ActionValue))))

(event Input|EnhancedActionEvents|EnhancedInputActionIA_ClickUI
  (params (ActionValue :type Boolean) (ElapsedSeconds :type Float%20%28double-precision%29) (TriggeredSeconds :type Float%20%28double-precision%29) (InputAction :type Input%20Action%20Object%20Reference :default "/Game/Input/IA_ClickUI.IA_ClickUI"))
  (:Started
    (Class|WidgetInteractionComponent|PressandReleaseKey (Variables|Default|GetWidgetInteraction) "Enter")))

(event Input|EnhancedActionEvents|EnhancedInputActionIA_ChangeObjectRotation
  (params (ActionValue :type Vector%202D%20Structure) (ElapsedSeconds :type Float%20%28double-precision%29) (TriggeredSeconds :type Float%20%28double-precision%29) (InputAction :type Input%20Action%20Object%20Reference :default "/Game/Input/IA_ChangeObjectRotation.IA_ChangeObjectRotation"))
  (bind _heldobject (Variables|Default|GetHeldObject)
    (:then
      (Transformation|SetActorRelativeRotation _heldobject (CallFunction|ThumbstickValuetoRotation ActionValue)))
    (:else)))

(event Input|EnhancedActionEvents|EnhancedInputActionIA_ResetObjectRotation
  (params (ActionValue :type Boolean) (ElapsedSeconds :type Float%20%28double-precision%29) (TriggeredSeconds :type Float%20%28double-precision%29) (InputAction :type Input%20Action%20Object%20Reference :default "/Game/Input/IA_ResetObjectRotation.IA_ResetObjectRotation"))
  (:Started
    (bind _heldobject (Variables|Default|GetHeldObject)
      (:then
        (Transformation|SetActorRelativeRotation _heldobject))
      (:else))))

(event Input|EnhancedActionEvents|EnhancedInputActionIA_Teleport
  (params (ActionValue :type Boolean) (ElapsedSeconds :type Float%20%28double-precision%29) (TriggeredSeconds :type Float%20%28double-precision%29) (InputAction :type Input%20Action%20Object%20Reference :default "/Game/Input/IA_Teleport.IA_Teleport"))
  (:Triggered
    (Utilities|FlowControl|DelayUntilNextTick)
    (bind (_traceendlocation _validforteleport) (CallFunction|TeleportTrace))
    (CallFunction|ShowTeleportLocation _traceendlocation _validforteleport))
  (:Started
    (Rendering|SetVisibility (Variables|Default|GetTeleportTraceEffect) true false))
  (:Completed
    (Rendering|SetVisibility (Variables|Default|GetTeleportRingEffect) false false)
    (if _validforteleport
      (Transformation|Teleport _traceendlocation (Transformation|GetActorRotation)))))

(event Input|EnhancedActionEvents|EnhancedInputActionIA_SnapTurn
  (params (ActionValue :type Float%20%28double-precision%29) (ElapsedSeconds :type Float%20%28double-precision%29) (TriggeredSeconds :type Float%20%28double-precision%29) (InputAction :type Input%20Action%20Object%20Reference :default "/Game/Input/IA_SnapTurn.IA_SnapTurn"))
  (:Started
    (Class|Actor|AddActorWorldRotation (Math|Rotator|MakeRotator 0.0 0.0 (* ActionValue (Variables|Default|GetSnapTurnAngle))) false true)))

(event Input|EnhancedActionEvents|EnhancedInputActionIA_HoldObject
  (params (ActionValue :type Boolean) (ElapsedSeconds :type Float%20%28double-precision%29) (TriggeredSeconds :type Float%20%28double-precision%29) (InputAction :type Input%20Action%20Object%20Reference :default "/Game/Input/IA_HoldObject.IA_HoldObject"))
  (:Started
    (Variables|Default|GetHeldObject
      (:then
        (CallFunction|ReleaseHeldObject))
      (:else
        (CallFunction|HoldHoveredObject)))))

(event Input|EnhancedActionEvents|EnhancedInputActionIA_Point
  (params (ActionValue :type Boolean) (ElapsedSeconds :type Float%20%28double-precision%29) (TriggeredSeconds :type Float%20%28double-precision%29) (InputAction :type Input%20Action%20Object%20Reference :default "/Game/Input/IA_Point.IA_Point"))
  (bind _pointtraceeffect (Variables|Default|GetPointTraceEffect))
  (:Triggered
    (Utilities|FlowControl|DelayUntilNextTick)
    (CallFunction|PointTrace))
  (:Started
    (Rendering|SetVisibility _pointtraceeffect true false))
  (:Completed
    (Rendering|SetVisibility _pointtraceeffect false false)
    (bind _hoveredobject (Variables|Default|GetHoveredObject)
      (:then
        (Class|InteractiveActor|SetState _hoveredobject "Free")
        (Variables|Default|SetHoveredObject 0))
      (:else))))

(event Input|EnhancedActionEvents|EnhancedInputActionIA_HandGrasp_L
  (params (ActionValue :type Float%20%28double-precision%29) (ElapsedSeconds :type Float%20%28double-precision%29) (TriggeredSeconds :type Float%20%28double-precision%29) (InputAction :type Input%20Action%20Object%20Reference :default "/Game/Input/IA_HandGrasp_L.IA_HandGrasp_L"))
  (bind _hand_l (Variables|Default|GetHand_L))
  (bind _returnvalue (Components|SkeletalMesh|GetAnimInstance _hand_l))
  (bind _asabp_mannequins_xr (Utilities|Casting|CastToABP_MannequinsXR _returnvalue))
  (:Triggered
    (Variables|/Game/Animations/ABP_MannequinsXR.ABP_MannequinsXR_C|SetPoseAlphaGrasp _asabp_mannequins_xr ActionValue))
  (:Completed
    (Variables|/Game/Animations/ABP_MannequinsXR.ABP_MannequinsXR_C|SetPoseAlphaGrasp _asabp_mannequins_xr 0.0)))

(event Input|EnhancedActionEvents|EnhancedInputActionIA_HandPoint_L
  (params (ActionValue :type Boolean) (ElapsedSeconds :type Float%20%28double-precision%29) (TriggeredSeconds :type Float%20%28double-precision%29) (InputAction :type Input%20Action%20Object%20Reference :default "/Game/Input/IA_HandPoint_L.IA_HandPoint_L"))
  (bind _hand_l (Variables|Default|GetHand_L))
  (bind _returnvalue (Components|SkeletalMesh|GetAnimInstance _hand_l))
  (bind _asabp_mannequins_xr (Utilities|Casting|CastToABP_MannequinsXR _returnvalue))
  (:Started
    (Variables|/Game/Animations/ABP_MannequinsXR.ABP_MannequinsXR_C|SetPoseAlphaPoint _asabp_mannequins_xr 0.0))
  (:Completed
    (Variables|/Game/Animations/ABP_MannequinsXR.ABP_MannequinsXR_C|SetPoseAlphaPoint _asabp_mannequins_xr 1.0)))

(event Input|EnhancedActionEvents|EnhancedInputActionIA_HandThumbUp_L
  (params (ActionValue :type Boolean) (ElapsedSeconds :type Float%20%28double-precision%29) (TriggeredSeconds :type Float%20%28double-precision%29) (InputAction :type Input%20Action%20Object%20Reference :default "/Game/Input/IA_HandThumbUp_L.IA_HandThumbUp_L"))
  (bind _hand_l (Variables|Default|GetHand_L))
  (bind _returnvalue (Components|SkeletalMesh|GetAnimInstance _hand_l))
  (bind _asabp_mannequins_xr (Utilities|Casting|CastToABP_MannequinsXR _returnvalue))
  (:Started
    (Variables|/Game/Animations/ABP_MannequinsXR.ABP_MannequinsXR_C|SetPoseAlphaThumbUp _asabp_mannequins_xr 0.0))
  (:Completed
    (Variables|/Game/Animations/ABP_MannequinsXR.ABP_MannequinsXR_C|SetPoseAlphaThumbUp _asabp_mannequins_xr 1.0)))

(event Input|EnhancedActionEvents|EnhancedInputActionIA_HandIndexCurl_R
  (params (ActionValue :type Float%20%28double-precision%29) (ElapsedSeconds :type Float%20%28double-precision%29) (TriggeredSeconds :type Float%20%28double-precision%29) (InputAction :type Input%20Action%20Object%20Reference :default "/Game/Input/IA_HandIndexCurl_R.IA_HandIndexCurl_R"))
  (bind _hand_r (Variables|Default|GetHand_R))
  (bind _returnvalue (Components|SkeletalMesh|GetAnimInstance _hand_r))
  (bind _asabp_mannequins_xr (Utilities|Casting|CastToABP_MannequinsXR _returnvalue))
  (:Triggered
    (Variables|/Game/Animations/ABP_MannequinsXR.ABP_MannequinsXR_C|SetPoseAlphaIndexCurl _asabp_mannequins_xr ActionValue))
  (:Completed
    (Variables|/Game/Animations/ABP_MannequinsXR.ABP_MannequinsXR_C|SetPoseAlphaIndexCurl _asabp_mannequins_xr 0.0)))

(event Input|EnhancedActionEvents|EnhancedInputActionIA_HandGrasp_R
  (params (ActionValue :type Float%20%28double-precision%29) (ElapsedSeconds :type Float%20%28double-precision%29) (TriggeredSeconds :type Float%20%28double-precision%29) (InputAction :type Input%20Action%20Object%20Reference :default "/Game/Input/IA_HandGrasp_R.IA_HandGrasp_R"))
  (bind _hand_r (Variables|Default|GetHand_R))
  (bind _returnvalue (Components|SkeletalMesh|GetAnimInstance _hand_r))
  (bind _asabp_mannequins_xr (Utilities|Casting|CastToABP_MannequinsXR _returnvalue))
  (:Triggered
    (Variables|/Game/Animations/ABP_MannequinsXR.ABP_MannequinsXR_C|SetPoseAlphaGrasp _asabp_mannequins_xr ActionValue))
  (:Completed
    (Variables|/Game/Animations/ABP_MannequinsXR.ABP_MannequinsXR_C|SetPoseAlphaGrasp _asabp_mannequins_xr 0.0)))

(event Input|EnhancedActionEvents|EnhancedInputActionIA_HandIndexCurl_L
  (params (ActionValue :type Float%20%28double-precision%29) (ElapsedSeconds :type Float%20%28double-precision%29) (TriggeredSeconds :type Float%20%28double-precision%29) (InputAction :type Input%20Action%20Object%20Reference :default "/Game/Input/IA_HandIndexCurl_L.IA_HandIndexCurl_L"))
  (bind _hand_l (Variables|Default|GetHand_L))
  (bind _returnvalue (Components|SkeletalMesh|GetAnimInstance _hand_l))
  (bind _asabp_mannequins_xr (Utilities|Casting|CastToABP_MannequinsXR _returnvalue))
  (:Triggered
    (Variables|/Game/Animations/ABP_MannequinsXR.ABP_MannequinsXR_C|SetPoseAlphaIndexCurl _asabp_mannequins_xr ActionValue))
  (:Completed
    (Variables|/Game/Animations/ABP_MannequinsXR.ABP_MannequinsXR_C|SetPoseAlphaIndexCurl _asabp_mannequins_xr 0.0)))

(event Input|EnhancedActionEvents|EnhancedInputActionIA_HandThumbUp_R
  (params (ActionValue :type Boolean) (ElapsedSeconds :type Float%20%28double-precision%29) (TriggeredSeconds :type Float%20%28double-precision%29) (InputAction :type Input%20Action%20Object%20Reference :default "/Game/Input/IA_HandThumbUp_R.IA_HandThumbUp_R"))
  (bind _hand_r (Variables|Default|GetHand_R))
  (bind _returnvalue (Components|SkeletalMesh|GetAnimInstance _hand_r))
  (bind _asabp_mannequins_xr (Utilities|Casting|CastToABP_MannequinsXR _returnvalue))
  (:Started
    (Variables|/Game/Animations/ABP_MannequinsXR.ABP_MannequinsXR_C|SetPoseAlphaThumbUp _asabp_mannequins_xr 0.0))
  (:Completed
    (Variables|/Game/Animations/ABP_MannequinsXR.ABP_MannequinsXR_C|SetPoseAlphaThumbUp _asabp_mannequins_xr 1.0)))

(event Input|EnhancedActionEvents|EnhancedInputActionIA_HandPoint_R
  (params (ActionValue :type Boolean) (ElapsedSeconds :type Float%20%28double-precision%29) (TriggeredSeconds :type Float%20%28double-precision%29) (InputAction :type Input%20Action%20Object%20Reference :default "/Game/Input/IA_HandPoint_R.IA_HandPoint_R"))
  (bind _hand_r (Variables|Default|GetHand_R))
  (bind _returnvalue (Components|SkeletalMesh|GetAnimInstance _hand_r))
  (bind _asabp_mannequins_xr (Utilities|Casting|CastToABP_MannequinsXR _returnvalue))
  (:Started
    (Variables|/Game/Animations/ABP_MannequinsXR.ABP_MannequinsXR_C|SetPoseAlphaPoint _asabp_mannequins_xr 0.0))
  (:Completed
    (Variables|/Game/Animations/ABP_MannequinsXR.ABP_MannequinsXR_C|SetPoseAlphaPoint _asabp_mannequins_xr 1.0)))

(fn ConstructionScript)

(fn AddSpawnableObjectstoUI
  (bind _widgetobject (Variables|Default|GetWidgetObject))
  (bind _spawnableobjects_combobox (Variables|/Game/Blueprints/WBP_UI.WBP_UI_C|GetSpawnableObjects_ComboBox _widgetobject))
  (for _array_element (Variables|Default|GetSpawnableObjects)
    (Class|ComboBoxString|AddOption _spawnableobjects_combobox (Utilities|Struct|BreakInteractiveActorData (Utilities|GetClassDefaults _array_element))))
  (Class|ComboBoxString|SetSelectedIndex _spawnableobjects_combobox))

(fn ThumbstickValuetoKeyboardKey
  (params (ActionValue :type Vector%202D%20Structure))
  (bind _returnvalue (Class|KismetMathLibrary|GetAbs2D ActionValue))
  (return (select (> (.x _returnvalue) (.y _returnvalue)) (select (> (.x ActionValue) 0.0) "Right" "Left") (select (> (.y ActionValue) 0.0) "Up" "Down"))))

(fn ResetWidgetFocus
  (Widget|SetFocus (Variables|Default|GetWidgetInteraction) (Variables|/Game/Blueprints/WBP_UI.WBP_UI_C|GetSpawnObject_Button (Variables|Default|GetWidgetObject)))
  (Class|WidgetInteractionComponent|PressandReleaseKey (Variables|Default|GetWidgetInteraction) "Right")
  (Class|WidgetInteractionComponent|PressandReleaseKey (Variables|Default|GetWidgetInteraction) "Left"))

(fn SpawnSelectedObject
  (params (ObjectIndex :type Integer))
  (Class|InteractiveActorsFunctions|SpawnInteractiveActor (Utilities|Array|Get(acopy) (Variables|Default|GetSpawnableObjects) ObjectIndex) (Transformation|GetWorldTransform (Variables|Default|GetSpawnedObjectPosition))))

(fn DestroyAvailableObject
  (bind _heldobject (Variables|Default|GetHeldObject)
    (:then
      (Class|InteractiveActorsFunctions|DestroyInteractiveActor _heldobject)
      (Variables|Default|SetHeldObject 0))
    (:else
      (bind _hoveredobject (Variables|Default|GetHoveredObject)
        (:then
          (Class|InteractiveActorsFunctions|DestroyInteractiveActor _hoveredobject)
          (Variables|Default|SetHoveredObject 0))
        (:else))))
  (Default|ClearDisplayedObject (Variables|Default|GetWidgetObject)))

(fn TeleportTrace
  (bind _motioncontrolleraim_l (Variables|Default|GetMotionControllerAim_L))
  (bind (_outhit _outpathpositions) (Class|GameplayStatics|BlueprintPredictProjectilePathbyObjectType (Transformation|GetWorldLocation _motioncontrolleraim_l) (* (Math|Vector|GetForwardVector _motioncontrolleraim_l) (Variables|Default|GetTeleportTraceProjectileSpeed)) true (Variables|Default|GetTeleportTraceProjectileRadius) (Utilities|Array|MakeArray "ObjectTypeQuery1") false 0 "None"))
  (bind _output_get (LocalVariables|SetPathPositions _outpathpositions))
  (Utilities|Array|Insert _output_get (Transformation|GetWorldLocation (Variables|Default|GetMotionControllerAim_L)))
  (Class|NiagaraDataInterfaceArrayFunctionLibrary|SetNiagaraArrayVector (Variables|Default|GetTeleportTraceEffect) "User.PointArray" (LocalVariables|GetPathPositions))
  (return (.ProjectedLocation (AI|Navigation|ProjectPointtoNavigation (Class|NavigationSystemV1|GetNavigationSystem) (.Location (Collision|BreakHitResult _outhit)) 0 0)) (.ReturnValue (AI|Navigation|ProjectPointtoNavigation (Class|NavigationSystemV1|GetNavigationSystem) (.Location (Collision|BreakHitResult _outhit)) 0 0))))

(fn ShowTeleportLocation
  (params (NewLocation :type Vector) (ValidForTeleport :type Boolean))
  (bind _teleportringeffect (Variables|Default|GetTeleportRingEffect))
  (Transformation|SetWorldLocation _teleportringeffect NewLocation false false)
  (if (!= ValidForTeleport (Rendering|IsVisible _teleportringeffect))
    (Rendering|SetVisibility (Variables|Default|GetTeleportRingEffect) ValidForTeleport false)))

(fn PointTrace
  (bind _motioncontrolleraim_r (Variables|Default|GetMotionControllerAim_R))
  (bind _returnvalue (Transformation|GetWorldLocation _motioncontrolleraim_r))
  (bind (_outhit _returnvalue_2) (Collision|LineTraceByChannel _returnvalue (+ _returnvalue (* (Math|Vector|GetForwardVector _motioncontrolleraim_r) (Variables|Default|GetPointTraceDistance))) "TraceTypeQuery1" false 0 "None"))
  (Class|NiagaraDataInterfaceArrayFunctionLibrary|SetNiagaraArrayVectorValue (Variables|Default|GetPointTraceEffect) "User.PointArray" 0 (.TraceStart (Collision|BreakHitResult _outhit)) false)
  (Class|NiagaraDataInterfaceArrayFunctionLibrary|SetNiagaraArrayVectorValue (Variables|Default|GetPointTraceEffect) "User.PointArray" 1 (select _returnvalue_2 (.Location (Collision|BreakHitResult _outhit)) (.TraceEnd (Collision|BreakHitResult _outhit))) false)
  (bind _asinteractive_actor (Utilities|Casting|CastToInteractiveActor (.HitActor (Collision|BreakHitResult _outhit)))
    (:then
      (if (!= _asinteractive_actor (Variables|Default|GetHoveredObject))
        (Utilities|FlowControl|Sequence
          (:then_0
            (bind _hoveredobject (Variables|Default|GetHoveredObject)
              (:then
                (Class|InteractiveActor|SetState _hoveredobject "Free"))
              (:else)))
          (:then_1
            (bind _output_get (Variables|Default|SetHoveredObject _asinteractive_actor))
            (Class|InteractiveActor|SetState _output_get "Hovered")
            (Default|DisplayNewObject (Variables|Default|GetWidgetObject) (Variables|/Script/VRDev_Vazhnov.InteractiveActor|GetData (Variables|Default|GetHoveredObject)))))))
    (:CastFailed
      (bind _hoveredobject_2 (Variables|Default|GetHoveredObject)
        (:then
          (Class|InteractiveActor|SetState _hoveredobject_2 "Free")
          (Variables|Default|SetHoveredObject 0)
          (Default|ClearDisplayedObject (Variables|Default|GetWidgetObject)))
        (:else)))))

(fn HoldHoveredObject
  (bind _hoveredobject (Variables|Default|GetHoveredObject)
    (:then
      (bind _output_get (Variables|Default|SetHeldObject _hoveredobject))
      (Class|InteractiveActor|SetState _output_get "Held")
      (Variables|Default|SetHoveredObject 0)
      (Default|DisplayNewObject (Variables|Default|GetWidgetObject) (Variables|/Script/VRDev_Vazhnov.InteractiveActor|GetData (Variables|Default|GetHeldObject)))
      (Transformation|AttachComponentToComponent (Variables|Default|GetHeldObject) (Variables|Default|GetHeldObjectPosition) "None" "SnapToTarget" "SnapToTarget" "KeepWorld" true)
      (Transformation|SetActorRelativeLocation (Variables|Default|GetHeldObject) (Math|Vector|MakeVector 0.0 (.SphereRadius (Collision|GetComponentBounds (Variables|/Script/Engine.StaticMeshActor|GetStaticMeshComponent (Variables|Default|GetHeldObject)))) 0.0)))
    (:else)))

(fn ReleaseHeldObject
  (Transformation|DetachFromActor (Variables|Default|GetHeldObject) "KeepWorld" "KeepWorld" "KeepWorld")
  (Class|InteractiveActor|SetState (Variables|Default|GetHeldObject) "Free")
  (Variables|Default|SetHeldObject 0)
  (Default|ClearDisplayedObject (Variables|Default|GetWidgetObject)))

(fn ThumbstickValuetoRotation
  (params (ActionValue :type Vector%202D%20Structure))
  (bind _heldobjectrotationspeed (Variables|Default|GetHeldObjectRotationSpeed))
  (bind _returnvalue (* ActionValue _heldobjectrotationspeed))
  (return (Class|KismetMathLibrary|QuatRotator (* (Math|Conversions|ToQuaternion(Rotator) (Math|Vector|RotatorfromAxisandAngle "0.000000,0.000000,1.000000" (.y _returnvalue))) (* (Math|Conversions|ToQuaternion(Rotator) (Math|Vector|RotatorfromAxisandAngle "1.000000,0.000000,0.000000" (.x _returnvalue))) (Math|Conversions|ToQuaternion(Rotator) (Variables|/Script/Engine.SceneComponent|GetRelativeRotation (Variables|/Script/Engine.Actor|GetRootComponent (Variables|Default|GetHeldObject)))))))))

(fn IsHoldingObject
  (return (Utilities|IsValid (Variables|Default|GetHeldObject))))

(fn IsHoveringObject
  (return (Utilities|IsValid (Variables|Default|GetHoveredObject))))

(fn IsWidgetShown
  (return (>= (Components|Timeline|GetPlaybackPosition (Variables|Default|GetWidgetScaleTimeline)) 0.1)))